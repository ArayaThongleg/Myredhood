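; BP_OutLine is a static prop that shows a colored outline while character_Redhhood overlaps its Box.
; On begin overlap it spawns a second, manually attached copy of its Mesh at the original's world transform, using a dynamic M_OutLine_Inst material.
; The material receives Color, but Scale is written to a parameter named None.
; End overlap destroys the copy, and HasOutLine guards against duplicates.
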(event `self.ReceiveBeginPlay`
  (`StaticMeshComponent.SetStaticMesh` (`self.StaticMesh`) (`self.Mesh`)))

(event `CreateOutLine`
  (if (not (`self.HasOutLine`))
    (bind _returnvalue (`AddComponent|NODE_AddStaticMeshComponent-0` :`bManualAttachment` true :`RelativeTransform` (`SceneComponent.K2_GetComponentToWorld` (`self.StaticMesh`))))
    (bind _output_get (set `self.Mesh Component` _returnvalue))
    (`StaticMeshComponent.SetStaticMesh` _output_get (`self.Mesh`))
    (bind _returnvalue_2 (`PrimitiveComponent.CreateDynamicMaterialInstance` _output_get 0 "/Game/OutLine_OBJECT/OutLineOBJ_UnMove/M_OutLine_Inst.M_OutLine_Inst" "None"))
    (`MaterialInstanceDynamic.SetVectorParameterValue` _returnvalue_2 "color" (`self.Color`))
    (`MaterialInstanceDynamic.SetScalarParameterValue` _returnvalue_2 "None" (`self.Scale`))
    (set `self.HasOutLine` true)))

(event `Delete Outline`
  (bind _mesh_component (`self.Mesh Component`))
  (`/Engine/EditorBlueprintResources/StandardMacros.IsValid` _mesh_component
    (:`Is Valid`
      (`ActorComponent.K2_DestroyComponent` _mesh_component)
      (set `self.HasOutLine` false))))

(event `self.Box.OnComponentBeginOverlap`
  (params (OverlappedComponent :type "PrimitiveComponent Object Reference") (OtherActor :type "Actor Object Reference") (OtherComp :type "PrimitiveComponent Object Reference") (OtherBodyIndex :type Integer) (bFromSweep :type Boolean) (SweepResult :type "HitResult Structure (by ref)"))
  (cast `/Game/RedhoodBP/character_Redhhood` OtherActor)
  (`self.CreateOutLine`))

(event `self.Box.OnComponentEndOverlap`
  (params (OverlappedComponent :type "PrimitiveComponent Object Reference") (OtherActor :type "Actor Object Reference") (OtherComp :type "PrimitiveComponent Object Reference") (OtherBodyIndex :type Integer))
  (cast `/Game/RedhoodBP/character_Redhhood` OtherActor)
  (`self.Delete Outline`))

(fn `UserConstructionScript`)