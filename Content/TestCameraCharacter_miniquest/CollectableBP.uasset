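; Collectable actor that the Redhhood character picks up by pressing E while inside its Box trigger.
; Overlap begin and end on the Box enable and disable the actor's input for player controller 0, so the key only responds in range.
; On pickup it decrements CollectablesLeft on the GM_Little game mode, adds a new Uitest widget to the viewport and destroys itself.
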(event `Key|E`
  (params (Key :type "Key Structure"))
  (:`Pressed`
    (bind _asgm_little (cast `/Game/TestCameraCharacter_miniquest/GM_Little` (`GameplayStatics.GetGameMode`)))
    (bind _result (`/Engine/EditorBlueprintResources/StandardMacros.DecrementInt` (`/Game/TestCameraCharacter_miniquest/GM_Little.CollectablesLeft` _asgm_little))
      (:`  `
        (set `/Game/TestCameraCharacter_miniquest/GM_Little.CollectablesLeft` _result _asgm_little)
        (bind _returnvalue (`|CreateWidget` "/Game/TestCameraCharacter_miniquest/uitest.uitest_C"))
        (`UserWidget.AddToViewport` _returnvalue 0)
        (`self.K2_DestroyActor`)))))

(event `self.Box.OnComponentBeginOverlap`
  (params (OverlappedComponent :type "PrimitiveComponent Object Reference") (OtherActor :type "Actor Object Reference") (OtherComp :type "PrimitiveComponent Object Reference") (OtherBodyIndex :type Integer) (bFromSweep :type Boolean) (SweepResult :type "HitResult Structure (by ref)"))
  (cast `/Game/TestCameraCharacter_miniquest/character_Redhhood` OtherActor)
  (`self.EnableInput` (`GameplayStatics.GetPlayerController` 0)))

(event `self.Box.OnComponentEndOverlap`
  (params (OverlappedComponent :type "PrimitiveComponent Object Reference") (OtherActor :type "Actor Object Reference") (OtherComp :type "PrimitiveComponent Object Reference") (OtherBodyIndex :type Integer))
  (cast `/Game/TestCameraCharacter_miniquest/character_Redhhood` OtherActor)
  (`self.DisableInput` (`GameplayStatics.GetPlayerController` 0)))

(fn `UserConstructionScript`)