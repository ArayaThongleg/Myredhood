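; Checkpoint actor that saves a respawn transform when the third-person character overlaps its trigger.
; On overlap, it loads the existing CheckPointSaveGame from its slot, or creates one if none exists.
; It stores its own location, raised along Z with zero rotation and unit scale, writes the save to the slot and prints the saved transform.
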(event `self.overlap.OnComponentBeginOverlap`
  (params (OverlappedComponent :type "PrimitiveComponent Object Reference") (OtherActor :type "Actor Object Reference") (OtherComp :type "PrimitiveComponent Object Reference") (OtherBodyIndex :type Integer) (bFromSweep :type Boolean) (SweepResult :type "HitResult Structure (by ref)"))
  (bind _returnvalue_location (`KismetMathLibrary.BreakTransform` (`self.GetTransform`)))
  (cast `/Game/ThirdPersonBP/Blueprints/ThirdPersonCharacter` OtherActor)
  (bind _returnvalue (`GameplayStatics.DoesSaveGameExist` (`self.Checkpoint SaveName`)))
  (if _returnvalue
    (bind _returnvalue_2 (`GameplayStatics.LoadGameFromSlot` (`self.Checkpoint SaveName`)))
    (bind _ascheck_point_save_game (cast `/Game/Checkpoint/CheckPointSaveGame` _returnvalue_2))
    (set `self.SaveGameReference` _ascheck_point_save_game)
    (else
      (bind _returnvalue_3 (`GameplayStatics.CreateSaveGameObject` "/Game/Checkpoint/CheckPointSaveGame.CheckPointSaveGame_C"))
      (set `self.SaveGameReference` _returnvalue_3)))
  (bind _output_get (set `/Game/Checkpoint/CheckPointSaveGame.Checkpoint` (`KismetMathLibrary.MakeTransform` (+ _returnvalue_location (0.0 0.0 200.0))) (`self.SaveGameReference`)))
  (`GameplayStatics.SaveGameToSlot` (`self.SaveGameReference`) (`self.Checkpoint SaveName`))
  (`KismetSystemLibrary.PrintString` (`KismetStringLibrary.Concat_StrStr` "Saved game" "Tranform :" (`KismetStringLibrary.Conv_TransformToString` _output_get))))

(fn `UserConstructionScript`)