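; GM_Little is a game mode that places the player at the door they came through and saves the current level.
; On BeginPlay it casts player character 0 to character_Redhhood and calls its SaveCurrentLevel.
; Its FindPlayerStart override picks the PlayerStart whose tag matches the DoorID stored in the MyGame_INT game instance, falling back to the first one found.
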(event `self.ReceiveBeginPlay`
  (bind _ascharacter_redhhood (cast `/Game/RedhoodBP/character_Redhhood` (`GameplayStatics.GetPlayerCharacter` 0)))
  (`/Game/RedhoodBP/character_Redhhood.Save Current Level` _ascharacter_redhhood))

(fn `FindPlayerStart`
  (params (Player :type "Controller Object Reference") (IncomingName :type String))
  (returns (ReturnValue :type "Actor Object Reference"))
  (bind _asmy_game_int (cast `/Game/Level_Travelling/MyGame_INT` (`GameplayStatics.GetGameInstance`)))
  (bind _outactors (`GameplayStatics.GetAllActorsOfClass` "/Script/Engine.PlayerStart"))
  (for _array_element _outactors
    (if (== (`/Game/Level_Travelling/MyGame_INT.DoorID` _asmy_game_int) (`PlayerStart.PlayerStartTag` _array_element))
      (return _array_element)))
  (return (`|GetArrayItem` _outactors)))

(fn `UserConstructionScript`)